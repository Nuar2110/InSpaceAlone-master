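; Generator actor that switches on through a TurnOn event, with no other active logic.
; TurnOn sets the IsHaveDiesel flag and turns the point light green.
; It then fades in three audio components in timed sequence using delays: the bottle sound, then the two generator sounds.
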(event Custom|TurnOn
  (Variables|Default|SetIsHaveDiesel true)
  (Rendering|Components|Light|SetLightColor (Variables|Default|GetPointLight) "(R=0.125059,G=1.000000,B=0.000000,A=1.000000)" true)
  (Audio|Components|Audio|FadeIn (Variables|Default|GetBottle) 0.0 1.0 0.0 "Linear" :!class /Script/Engine.AudioComponent)
  (Utilities|FlowControl|Delay 3.0)
  (Audio|Components|Audio|FadeIn (Variables|Default|GetGenerator) 0.0 1.0 0.0 "Linear" :!class /Script/Engine.AudioComponent)
  (Utilities|FlowControl|Delay 2.8096)
  (Audio|Components|Audio|FadeIn (Variables|Default|GetGenerator2) 0.0 1.0 0.0 "Linear" :!class /Script/Engine.AudioComponent))

(event EventBeginPlay)

(event Collision|EventActorBeginOverlap
  (params (OtherActor :type Actor%20Object%20Reference)))

(event EventTick
  (params (DeltaSeconds :type Float%20%28single-precision%29)))

(fn ConstructionScript)