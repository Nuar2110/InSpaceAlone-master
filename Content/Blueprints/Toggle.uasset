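; Toggle switch actor that flips between an up and a down state through two custom events, TurnUp and TurnDown.
; Each event snaps PivotPoint to an opposite tilt, sets IsTurnedUp, recolors the PointLight green for up or red for down, and fades in its own component, Toggle1 or Toggle2.
; Nothing in this Blueprint calls the events, and it runs no Tick or BeginPlay logic.
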(event Custom|TurnUp
  (Transformation|SetRelativeRotation (Variables|Default|GetPivotPoint) "0, 0,30.000000" false false)
  (Variables|Default|SetIsTurnedUp true)
  (Rendering|Components|Light|SetLightColor (Variables|Default|GetPointLight) "(R=0.084376,G=1.000000,B=0.000000,A=1.000000)" true)
  (Audio|Components|Audio|FadeIn (Variables|Default|GetToggle1) 0.0 1.0 0.0 "Linear" :!class /Script/Engine.AudioComponent))

(event Custom|TurnDown
  (Transformation|SetRelativeRotation (Variables|Default|GetPivotPoint) "0, 0,-30.000000" false false)
  (Variables|Default|SetIsTurnedUp false)
  (Rendering|Components|Light|SetLightColor (Variables|Default|GetPointLight) "(R=1.000000,G=0.054480,B=0.000000,A=1.000000)" true)
  (Audio|Components|Audio|FadeIn (Variables|Default|GetToggle2) 0.0 1.0 0.0 "Linear" :!class /Script/Engine.AudioComponent))

(event EventBeginPlay)

(event Collision|EventActorBeginOverlap
  (params (OtherActor :type Actor%20Object%20Reference)))

(event EventTick
  (params (DeltaSeconds :type Float%20%28single-precision%29)))

(fn ConstructionScript)