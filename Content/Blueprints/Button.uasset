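; Button actor with a light and a pressable cylinder that handles the end-of-game sequence.
; Its EndGame event clears IsNeedGG, turns the point light green, fades in the Pizza component and lowers the cylinder.
; After a short delay it opens the "Game" level.
; Disconnected nodes for raising and repositioning a Door remain in the graph but never run.
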(event Custom|EndGame
  (Variables|Default|SetIsNeedGG false)
  (Rendering|Components|Light|SetLightColor (Variables|Default|GetPointLight) "(R=0.105700,G=1.000000,B=0.000000,A=1.000000)" true)
  (Audio|Components|Audio|FadeIn (Variables|Default|GetPizza) 0.0 1.0 0.0 "Linear" :!class /Script/Engine.AudioComponent)
  (Transformation|AddLocalOffset (Variables|Default|GetCylinder) "0, 0,-6.000000" false false)
  (Utilities|FlowControl|Delay 1.5)
  (Game|OpenLevel(byName) "Game"))

(event EventBeginPlay)

(event Collision|EventActorBeginOverlap
  (params (OtherActor :type Actor%20Object%20Reference)))

(event EventTick
  (params (DeltaSeconds :type Float%20%28single-precision%29)))

(fn ConstructionScript)